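; Inventory component for a horror game, storing items in a slot array filled with empty entries at BeginPlay.
; Add, remove, count and swap functions edit the slots, with stack limits read from an item data table.
; UseItem removes one unit of any type, but only consumables have effects, restoring the horror character's health, sanity and battery; other types just print.
; DropItem line-traces for ground ahead of the player, spawns a BP_WorldItem and empties the slot.
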(event EventBeginPlay
  (Setup|InitializeInventory))

(fn InitializeInventory
  (for _index (range 0 (LocalVariables|GetInventorySize))
    (Utilities|Array|Add (Variables|Default|GetInventory) (Utilities|Struct|MakeFInventorySlot "None" 0 true))))

(fn AddItem
  (params (ItemID :type Name) (Amount :type Integer))
  (if (<= Amount 0)
    (return false)
    (else
      (bind _returnvalue (Utilities|GetDataTableRow (Variables|Default|GetItems_DataTable) ItemID)
        (:then
          (LocalVariables|SetRemainingAmount Amount)
          (if (.bIsStackable (Utilities|Struct|BreakFItemData _returnvalue))
            (for (_array_element _array_index) (Variables|Default|GetInventory)
              (if (and (and (== (.bIsEmpty (Utilities|Struct|BreakFInventorySlot _array_element)) false) (== (.ItemID (Utilities|Struct|BreakFInventorySlot _array_element)) ItemID)) (< (.Quantity (Utilities|Struct|BreakFInventorySlot _array_element)) (.MaxStackSize (Utilities|Struct|BreakFItemData _returnvalue))))
                (LocalVariables|SetSpaceLeft (- (.MaxStackSize (Utilities|Struct|BreakFItemData _returnvalue)) (.Quantity (Utilities|Struct|BreakFInventorySlot _array_element))))
                (LocalVariables|SetAmoutToAdd (Math|Integer|Min(Integer) (LocalVariables|GetRemainingAmount) (LocalVariables|GetSpaceLeft)))
                (LocalVariables|SetNewQuantity (+ (.Quantity (Utilities|Struct|BreakFInventorySlot _array_element)) (LocalVariables|GetAmoutToAdd)))
                (LocalVariables|SetRemainingAmount (- (LocalVariables|GetRemainingAmount) (LocalVariables|GetAmoutToAdd)))
                (bind _structout (Utilities|Struct|SetmembersinFInventorySlot _array_element (.ItemID (Utilities|Struct|BreakFInventorySlot _array_element)) (LocalVariables|GetNewQuantity) false))
                (Utilities|Array|SetArrayElem (Variables|Default|GetInventory) _array_index _structout)
                (if (not (> (LocalVariables|GetRemainingAmount) 0))
                  (return true)))))
          (for (_array_element_2 _array_index_2) (Variables|Default|GetInventory)
            (if (.bIsEmpty (Utilities|Struct|BreakFInventorySlot _array_element_2))
              (if (.bIsStackable (Utilities|Struct|BreakFItemData _returnvalue))
                (LocalVariables|SetAmoutToAdd (Math|Integer|Min(Integer) (LocalVariables|GetRemainingAmount) (.MaxStackSize (Utilities|Struct|BreakFItemData _returnvalue))))
                (else
                  (LocalVariables|SetAmoutToAdd 1)))
              (LocalVariables|SetRemainingAmount (- (LocalVariables|GetRemainingAmount) (LocalVariables|GetAmoutToAdd)))
              (bind _structout_2 (Utilities|Struct|SetmembersinFInventorySlot _array_element_2 ItemID (LocalVariables|GetAmoutToAdd) false))
              (Utilities|Array|SetArrayElem (Variables|Default|GetInventory) _array_index_2 _structout_2)
              (if (not (> (LocalVariables|GetRemainingAmount) 0))
                (return true))))
          (return false))
        (:RowNotFound
          (return false))))))

(fn RemoveItem
  (params (ItemID :type Name) (Amount :type Integer))
  (if (<= Amount 0)
    (return false)
    (else
      (LocalVariables|SetRemainingAmount Amount)
      (for (_array_element _array_index) (Variables|Default|GetInventory)
        (if (and (> (.Quantity (Utilities|Struct|BreakFInventorySlot _array_element)) 0) (and (== ItemID (.ItemID (Utilities|Struct|BreakFInventorySlot _array_element))) (not (.bIsEmpty (Utilities|Struct|BreakFInventorySlot _array_element)))))
          (LocalVariables|SetNewQuantity (- (.Quantity (Utilities|Struct|BreakFInventorySlot _array_element)) (Math|Integer|Min(Integer) (.Quantity (Utilities|Struct|BreakFInventorySlot _array_element)) (LocalVariables|GetRemainingAmount))))
          (LocalVariables|SetRemainingAmount (- (LocalVariables|GetRemainingAmount) (Math|Integer|Min(Integer) (.Quantity (Utilities|Struct|BreakFInventorySlot _array_element)) (LocalVariables|GetRemainingAmount))))
          (if (<= (LocalVariables|GetNewQuantity) 0)
            (bind _structout (Utilities|Struct|SetmembersinFInventorySlot _array_element "None" 0 true))
            (Utilities|Array|SetArrayElem (Variables|Default|GetInventory) _array_index _structout)
            (else
              (bind _structout_2 (Utilities|Struct|SetmembersinFInventorySlot _array_element (.ItemID (Utilities|Struct|BreakFInventorySlot _array_element)) (LocalVariables|GetNewQuantity) false))
              (Utilities|Array|SetArrayElem (Variables|Default|GetInventory) _array_index _structout_2)))
          (if (<= (LocalVariables|GetRemainingAmount) 0)
            (return true))))
      (return false))))

(fn UseItem
  (params (SlotIndex :type Integer))
  (bind _inventory (Variables|Default|GetInventory))
  (bind _output (Utilities|Array|Get(acopy) _inventory SlotIndex))
  (bind (_itemid _quantity _bisempty) (Utilities|Struct|BreakFInventorySlot _output))
  (if (Utilities|Array|IsValidIndex (Variables|Default|GetInventory) SlotIndex)
    (if _bisempty
      (return)
      (else
        (bind _returnvalue (Utilities|GetDataTableRow "/Game/DarkwoodDescent/Blueprints/Data/DT_Items.DT_Items" _itemid)
          (:then
            (LocalVariables|SetItem _returnvalue)
            (switch Utilities|FlowControl|Switch|SwitchonEItemType (.itemtype (LocalVariables|GetItem))
              (:NewEnumerator0
                (CallFunction|UseConsumable (LocalVariables|GetItem)))
              (:NewEnumerator1
                (Development|PrintString "[AC_INVENTORY] UseItem - Key Item" true true "(R=0.723265,G=1.000000,B=0.003448,A=1.000000)" 1e+01))
              (:NewEnumerator2
                (Development|PrintString "[AC_INVENTORY] UseItem - Document Item" true true "(R=0.723265,G=1.000000,B=0.003448,A=1.000000)" 1e+01))
              (:NewEnumerator3
                (Development|PrintString "[AC_INVENTORY] UseItem - Weapon Item" true true "(R=0.723265,G=1.000000,B=0.003448,A=1.000000)" 1e+01))
              (:NewEnumerator4
                (Development|PrintString "[AC_INVENTORY] UseItem - Craft Item" true true "(R=0.723265,G=1.000000,B=0.003448,A=1.000000)" 1e+01)))
            (bind _success (Core|RemoveItem _itemid 1))
            (if _success
              (Development|PrintString "[AC_INVENTORY] UseItem - Remove Item OK" true true "(R=0.121437,G=1.000000,B=0.000000,A=1.000000)" 1e+01)
              (else
                (Development|PrintString "[AC_INVENTORY] UseItem - Remove Item NOK" true true "(R=1.000000,G=0.006130,B=0.000000,A=1.000000)" 1e+01))))
          (:RowNotFound
            (return)))))
    (else
      (return))))

(fn DropItem
  (params (SlotIndex :type Integer))
  (bind _returnvalue (Game|GetPlayerCharacter 0))
  (bind _returnvalue_2 (Math|Vector|MakeVector 0.0 0.0 2e+01))
  (bind _inventory (Variables|Default|GetInventory))
  (bind _multiplyvalue (LocalVariables|GetMultiplyValue))
  (bind _returnvalue_3 (Transformation|GetActorLocation _returnvalue))
  (bind _returnvalue_4 (Transformation|GetActorForwardVector _returnvalue))
  (bind _output (Utilities|Array|Get(acopy) _inventory SlotIndex))
  (bind (_itemid _quantity _bisempty) (Utilities|Struct|BreakFInventorySlot _output))
  (bind _returnvalue_5 (* _returnvalue_4 _multiplyvalue))
  (bind _returnvalue_6 (+ _returnvalue_3 _returnvalue_5))
  (bind _returnvalue_7 (+ _returnvalue_6 _returnvalue_2))
  (if (Utilities|Array|IsValidIndex (Variables|Default|GetInventory) SlotIndex)
    (if _bisempty
      (return)
      (else
        (bind (_outhit _returnvalue_8) (Collision|LineTraceByChannel (+ _returnvalue_7 "0.000000,0.000000,100.000000") (- _returnvalue_7 "0.000000,0.000000,1000.000000") "TraceTypeQuery1" false 0 "None"))
        (if _returnvalue_8
          (LocalVariables|SetDropLocation (+ (.ImpactPoint (Collision|BreakHitResult _outhit)) "0.000000,0.000000,5.000000"))
          (else
            (LocalVariables|SetDropLocation _returnvalue_7)))
        (bind _returnvalue_9 (Utilities|GetDataTableRow "/Game/DarkwoodDescent/Blueprints/Data/DT_Items.DT_Items" _itemid)
          (:then
            (bind _returnvalue_10 (Game|SpawnActorfromClass "/Game/DarkwoodDescent/Blueprints/Items/BP_WorldItem.BP_WorldItem_C" (Math|Transform|MakeTransform (LocalVariables|GetDropLocation) (Transformation|GetActorRotation _returnvalue) (Math|Conversions|ToVector(Float) (.worldscale _returnvalue_9))) "Undefined" "MultiplyWithRoot" 0 _itemid _quantity 0))
            (Components|StaticMesh|SetStaticMesh (Variables|/Game/DarkwoodDescent/Blueprints/Items/BP_WorldItem.BP_WorldItem_C|GetStaticMesh _returnvalue_10) (.mesh _returnvalue_9))
            (bind _structout (Utilities|Struct|SetmembersinFInventorySlot _output "None" 0 true))
            (Utilities|Array|SetArrayElem (Variables|Default|GetInventory) SlotIndex _structout)))))
    (else
      (return))))

(fn HasItem
  (params (ItemName :type Name))
  (for _array_element (Variables|Default|GetInventory)
    (if (and (> (.Quantity (Utilities|Struct|BreakFInventorySlot _array_element)) 0) (== (== ItemName (.ItemID (Utilities|Struct|BreakFInventorySlot _array_element))) (not (.bIsEmpty (Utilities|Struct|BreakFInventorySlot _array_element)))))
      (return true)))
  (return false))

(fn GetItemCount
  (params (ItemIDName :type Name))
  (bind _hasitem (Queries|HasItem ItemIDName))
  (if _hasitem
    (for _array_element (Variables|Default|GetInventory)
      (if (== ItemIDName (.ItemID (Utilities|Struct|BreakFInventorySlot _array_element)))
        (LocalVariables|SetCountAmount (+ (.Quantity (Utilities|Struct|BreakFInventorySlot _array_element)) (LocalVariables|GetCountAmount)))))
    (return (LocalVariables|GetCountAmount))
    (else
      (return 0))))

(fn FindEmptySlot
  (for (_array_element _array_index) (Variables|Default|GetInventory)
    (if (.bIsEmpty (Utilities|Struct|BreakFInventorySlot _array_element))
      (return _array_index)))
  (return -1))

(fn SwapSlot
  (params (IndexA :type Integer) (IndexB :type Integer))
  (bind _inventory (Variables|Default|GetInventory))
  (if (and (Utilities|Array|IsValidIndex (Variables|Default|GetInventory) IndexA) (Utilities|Array|IsValidIndex (Variables|Default|GetInventory) IndexB))
    (if (== IndexA IndexB)
      (return)
      (else
        (LocalVariables|SetSlotA (Utilities|Array|Get(acopy) (Variables|Default|GetInventory) IndexA))
        (LocalVariables|SetSlotB (Utilities|Array|Get(acopy) (Variables|Default|GetInventory) IndexB))
        (Utilities|Array|SetArrayElem _inventory IndexA (LocalVariables|GetSlotB))
        (Utilities|Array|SetArrayElem _inventory IndexB (LocalVariables|GetSlotA))))
    (else
      (return))))

(fn GetItem
  (params (SlotIndex :type Integer))
  (bind _inventory (Variables|Default|GetInventory))
  (if (Utilities|Array|IsValidIndex _inventory SlotIndex)
    (return (Utilities|Array|Get(acopy) _inventory SlotIndex) true)
    (else
      (return "" false))))

(fn UseConsumable
  (params (ItemRef :type F%20Item%20Data%20Structure))
  (bind _asbp_horror_character (Utilities|Casting|CastToBP_HorrorCharacter (Components|GetOwner)))
  (Default|AddHealth _asbp_horror_character (.healthrestore ItemRef))
  (Default|AddSanity _asbp_horror_character (.sanityrestore ItemRef))
  (Default|AddBattery _asbp_horror_character (.batteryrestore ItemRef))
  (Default|UpdateBattery (Variables|/Game/DarkwoodDescent/Blueprints/BP_HorrorCharacter.BP_HorrorCharacter_C|GetHUDFlashlightRef _asbp_horror_character) (Variables|/Game/DarkwoodDescent/Blueprints/BP_HorrorCharacter.BP_HorrorCharacter_C|GetCurrentBattery _asbp_horror_character) (Variables|/Game/DarkwoodDescent/Blueprints/BP_HorrorCharacter.BP_HorrorCharacter_C|GetMaxBattery _asbp_horror_character)))