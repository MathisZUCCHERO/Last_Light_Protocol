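; BP_Door is an interactable hinged door that opens and closes with creak sounds.
; Interact flips IsOpen and plays or reverses the TL_OpenDoor timeline, which lerps the DoorHinge yaw between zero and OpenAngle.
; When RequiresKey is set it only prints "Locked", with no key check or unlock logic here.
; GetInteractPrompt returns Locked, Open Door or Close Door to match the current state.
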(event EventInteract
  (params (Caller :type Actor%20Object%20Reference))
  (bind _returnvalue (Transformation|GetActorLocation))
  (if (Variables|Default|GetbRequiresKey)
    (Development|PrintString "Locked")
    (elif (Variables|Default|GetbIsOpen)
      (Audio|PlaySoundatLocation (Variables|Default|GetCloseDoorCreakSound) _returnvalue "0, 0, 0" 0.5 1.0 0.0 0 0 0 0)
      (Variables|Default|SetbIsOpen false)
      (bind _alpha (Timeline|TL_OpenDoor Reverse)
        (:Update
          (Transformation|SetRelativeRotation (Variables|Default|GetDoorHinge) (Math|Rotator|MakeRotator 0.0 0.0 (Math|Float|Lerp 0.0 (Variables|Default|GetOpenAngle) _alpha)) false false)))
      (else
        (Audio|PlaySoundatLocation (Variables|Default|GetOpenDoorCreakSound) _returnvalue "0, 0, 0" 0.5 1.0 0.0 0 0 0 0)
        (Variables|Default|SetbIsOpen true)
        (Timeline|TL_OpenDoor Play)))))

(fn ConstructionScript)

(fn GetInteractPrompt
  (if (Variables|Default|GetbRequiresKey)
    (return "Locked")
    (elif (Variables|Default|GetbIsOpen)
      (return "Close Door")
      (else
        (return "Open Door")))))